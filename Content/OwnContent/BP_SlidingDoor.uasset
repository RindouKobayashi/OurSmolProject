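; BP_SlidingDoor is an interactable door that slides open and closed along its local Y axis.
; Interact is ignored while the timeline plays, otherwise a FlipFlop alternates playing and reversing it.
; The timeline's alpha lerps the door mesh from a fixed closed offset to DoorSlideOpen.
; SetDoorOpen picks a signed DoorOpenAngle from the player's side using a dot product, but the slide logic never uses it.
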(event `self.Interact`
  (params (`Player Location` :type "Vector Structure") (Player :type "/Game/ThirdPerson/Blueprints/BP_ThirdPersonCharacter Object Reference") (IsHolding :type Boolean))
  ;[1 1 1] Door Code
  (if (not (`TimelineComponent.IsPlaying` (`self.Door Timeline`)))
    (`/Engine/EditorBlueprintResources/StandardMacros.FlipFlop`
      (:`A`
        (bind (_direction _dooralpha) (`Timeline|Door Timeline` :!label _label)
          (:`Update`
            (`SceneComponent.K2_SetRelativeLocation` (`self.Door`) (`KismetMathLibrary.MakeVector` 0.0 (`KismetMathLibrary.Lerp` 44.0 (`self.Door Slide Open`) _dooralpha)) false false))))
      (:`B`
        (goto _label :!via `Reverse`)))))

(fn `Set Door Open`
  (params (PlayerLocation :type "Vector Structure"))
  ;[1 1 1] Calculate Door Angle based on a dot product
  (set `self.DoorOpenAngle` (`KismetMathLibrary.SelectFloat` -90.0 90.0 (>= (`KismetMathLibrary.Dot_VectorVector` (`KismetMathLibrary.GetDirectionUnitVector` (`self.K2_GetActorLocation`) PlayerLocation) (`self.GetActorForwardVector`)) 0.0)))
  (return))

(fn `UserConstructionScript`)