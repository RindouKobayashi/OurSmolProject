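; BP_DoubleDoor is an interactable door actor that swings open away from or toward a side chosen by the player's position, then closes on the next interaction.
; Interact is ignored while DoorTimeline plays, otherwise a FlipFlop alternates between playing and reversing it.
; On opening, SetDoorOpenAngle uses a forward-vector dot product to pick the swing sign.
; The timeline alpha lerps DoorLeft's yaw; no other leaf is rotated.
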(event `self.Interact`
  (params (`Player Location` :type "Vector Structure") (Player :type "/Game/ThirdPerson/Blueprints/BP_ThirdPersonCharacter Object Reference") (IsHolding :type Boolean))
  ;[1 1 1] Door Code
  (if (not (`TimelineComponent.IsPlaying` (`self.Door Timeline`)))
    (`/Engine/EditorBlueprintResources/StandardMacros.FlipFlop`
      (:`A`
        (`self.SetDoorOpenAngle` `Player Location`)
        (bind (_direction _dooralpha) (`Timeline|Door Timeline` :!label _label)
          (:`Update`
            (`SceneComponent.K2_SetRelativeRotation` (`self.Door Left`) (`KismetMathLibrary.MakeRotator` 0.0 0.0 (`KismetMathLibrary.Lerp` 0.0 (`self.DoorOpenAngle`) _dooralpha)) false false))))
      (:`B`
        (goto _label :!via `Reverse`)))))

(fn `SetDoorOpenAngle`
  (params (PlayerLocation :type "Vector Structure"))
  ;[1 1 1] Calculate Door Angle based on a dot product
  (set `self.DoorOpenAngle` (`KismetMathLibrary.SelectFloat` -90.0 90.0 (>= (`KismetMathLibrary.Dot_VectorVector` (`KismetMathLibrary.GetDirectionUnitVector` (`self.K2_GetActorLocation`) PlayerLocation) (`self.GetActorForwardVector`)) 0.0)))
  (return))

(fn `UserConstructionScript`)